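; ConstructionProxy is a ghost-material placeholder actor that times a construction job and removes itself when it finishes.
; It binds to the game state's game speed update, with a time unit feeding the clockwork accumulated each tick.
; Once work time reaches the construction time set from work hours, it signals completion with itself and destroys itself after a short delay.
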(event Custom|AdjusteTime
  (params (TimeUnit :type Float%20%28single-precision%29))
  (Variables|Default|SetTimeUnit TimeUnit))

(event EventBeginPlay
  (bind _output_get (Variables|Default|SetGameStateRef (.AsMy%20Game%20State%20Base (Utilities|Casting|CastToMyGameStateBase (Game|GetGameState)))))
  (EventDispatchers|BindEventtoUpdateGameSpeed _output_get (EventDispatchers|CreateEvent :!event Custom|AdjusteTime)))

(event EventTick
  (params (DeltaSeconds :type Float%20%28single-precision%29))
  (Variables|Default|SetDelta DeltaSeconds)
  (if (not (Variables|Default|GetIsConstructionCompleted))
    (CallFunction|DoWork)
    (if (>= (Variables|Default|GetWorkTimeSpent) (Variables|Default|GetConstructionTime))
      (Variables|Default|SetIsConstructionCompleted true)
      (Default|CallConstructionCompleted self)
      (Utilities|FlowControl|Delay 0.2)
      (Actor|DestroyActor))))

(fn ConstructionScript
  (bind _staticmesh (Variables|Default|GetStaticMesh))
  (Components|StaticMesh|SetStaticMesh _staticmesh (Variables|Default|GetDisplayMesh))
  (Rendering|Material|SetMaterial _staticmesh 0 "/Game/Materials/Ghost_M_Inst.Ghost_M_Inst"))

(fn SetConstructionTime
  (params (WorkHours :type Float%20%28single-precision%29))
  (Variables|Default|SetConstructionTime (* WorkHours 6e+01))
  (return))

(fn DoWork
  (bind _output_get (Variables|Default|SetClockwork (.ClockWorkOut (CallFunction|SetClockWork (Variables|Default|GetDelta) (Variables|Default|GetTimeUnit) (Variables|Default|GetClockwork)))))
  (Variables|Default|SetWorkTimeSpent (* _output_get 6e+01))
  (return))