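; ConstructionManager_BP manages building construction by placing proxy actors that are replaced with real buildings when work completes.
; QueueConstruction spawns a proxy with a display mesh and required work hours, binds its completion event, and stores it and its config in parallel arrays.
; On completion, FinishConstruction looks up the config by the proxy's index, removes both entries, spawns the building at the saved transform and destroys the proxy.
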(event Custom|BindConstuctionComplete
  (params (Proxy :type Construction%20Proxy%20Object%20Reference))
  (EventDispatchers|BindEventtoConstructionCompleted Proxy (EventDispatchers|CreateEvent :!event Custom|ConstructionCompeted)))

(event Custom|ConstructionCompeted
  (params (Proxy :type Construction%20Proxy%20Object%20Reference))
  (CallFunction|FinishConstruction Proxy))

(fn ConstructionScript)

(fn QueueConstruction
  (params (ConstructionStruct :type Construction%20Struc%20Structure))
  (bind (_buildingclass _proxyclass _transform _displaymesh _workhoursrequired) (Utilities|Struct|BreakConstruction_Struc ConstructionStruct))
  (bind _returnvalue (Game|SpawnActorfromClass _proxyclass _transform "Undefined" 0 _displaymesh 0))
  (CallFunction|BindConstuctionComplete _returnvalue)
  (Utilities|Array|Add (Variables|Default|GetProxies) _returnvalue)
  (Utilities|Array|Add (Variables|Default|GetQueue) ConstructionStruct)
  (Default|SetConstructionTime _returnvalue _workhoursrequired))

(fn FinishConstruction
  (params (Proxy :type Construction%20Proxy%20Object%20Reference))
  (bind _proxies (Variables|Default|GetProxies))
  (bind _output_get (Variables|Default|SetIndex (Utilities|Array|FindItem _proxies Proxy)))
  (Variables|Default|SetConfig (Utilities|Array|Get(acopy) (Variables|Default|GetQueue) _output_get))
  (Utilities|Array|RemoveIndex (Variables|Default|GetQueue) (Variables|Default|GetIndex))
  (Utilities|Array|RemoveIndex _proxies (Variables|Default|GetIndex))
  (Game|SpawnActorfromClass (.BuildingClass (Utilities|Struct|BreakConstruction_Struc (Variables|Default|GetConfig))) (.Transform (Utilities|Struct|BreakConstruction_Struc (Variables|Default|GetConfig))) "AlwaysSpawn" 0 0 0)
  (Actor|DestroyActor Proxy))