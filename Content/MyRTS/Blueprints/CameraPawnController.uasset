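; RTS player controller that drives the camera pawn and building placement.
; BeginPlay caches pawn and game state, spawns the construction manager and ghost building, and creates the main HUD.
; Input moves the camera with zoom-scaled speed, edge scrolling, gated mouse rotation and clamped spring-arm zoom.
; In build mode the ghost follows the cursor and rotates; left-click queues non-overlapping placements, while V spawns an NPC at the cursor.
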(event EventBeginPlay
  (bind _returnvalue (Math|Transform|MakeTransform "0, 0, 0"))
  (bind _camerapawnref (Variables|References|GetCameraPawnRef))
  ;[1 1 1] BeginPlay
  (Utilities|FlowControl|Sequence
    (:then_0
      (Utilities|ReferenceCasts))
    (:then_1
      (bind _returnvalue_2 (Game|SpawnActorfromClass "/Game/MyRTS/Blueprints/Construction/ConstructionManager_BP.ConstructionManager_BP_C" _returnvalue "AlwaysSpawn" 0 0))
      (Variables|References|SetConstrucionManagerRef _returnvalue_2))
    (:then_2
      (bind _returnvalue_3 (Game|SpawnActorfromClass "/Game/MyRTS/Blueprints/Buildings/GhostBuilding_Bp.GhostBuilding_Bp_C" _returnvalue "AlwaysSpawn" 0 self 0))
      (Variables|References|SetGhostBuildingRef _returnvalue_3))
    (:then_3
      (Variables|/Script/Engine.SpringArmComponent|SetTargetArmLength (Variables|/Game/MyRTS/Blueprints/CameraPawn.CameraPawn_C|GetSpringArm _camerapawnref) (Variables|/Game/MyRTS/Blueprints/CameraPawn.CameraPawn_C|GetArmLenghtDefault _camerapawnref))
      (Input|SetInputModeGameandUI self 0 "DoNotLock" false)
      (Utilities|CreateHuds)
      (UserInterface|Viewport|AddtoViewport (Variables|References|GetMainHud_Ref) 0))))

(event EventTick
  (params (DeltaSeconds :type Float%20%28single-precision%29))
  (if (Variables|Default|GetBuildModeActive)
    (|SetCursorWordPostion)))

(event Input|ActionEvents|InputActionPan
  (params (Key :type Key%20Structure))
  (bind _camerapawnref (Variables|References|GetCameraPawnRef))
  (bind _returnvalue (Transformation|GetActorRotation _camerapawnref))
  (bind (_roll _pitch _yaw) (Math|Rotator|BreakRotator _returnvalue))
  ;[1 1 1] Pan Y
  (:Pressed
    (Variables|Default|SetDisableCamNav true)
    (Utilities|FlowControl|Gate true) ; enters at Open
  )
  (:Released
    (Variables|Default|SetDisableCamNav false)
    (Utilities|FlowControl|Gate true) ; enters at Close
  ))

(event Input|ActionEvents|InputActionPan
  (params (Key :type Key%20Structure))
  (bind _camerapawnref (Variables|References|GetCameraPawnRef))
  (bind _returnvalue (Transformation|GetActorRotation _camerapawnref))
  (bind (_roll _pitch _yaw) (Math|Rotator|BreakRotator _returnvalue))
  ;[1 1 1] Pan X
  (:Pressed
    (Variables|Default|SetDisableCamNav true)
    (Utilities|FlowControl|Gate true) ; enters at Open
  )
  (:Released
    (Variables|Default|SetDisableCamNav false)
    (Utilities|FlowControl|Gate true) ; enters at Close
  ))

(event Input|ActionEvents|InputActionPanReset
  (params (Key :type Key%20Structure))
  (bind _camerapawnref (Variables|References|GetCameraPawnRef))
  (bind _returnvalue (Transformation|GetActorRotation _camerapawnref))
  (bind (_roll _pitch _yaw) (Math|Rotator|BreakRotator _returnvalue))
  ;[1 1 1] Pan Reset
  (:Pressed
    (Transformation|SetActorRotation _camerapawnref (Math|Rotator|MakeRotator _roll 0.0 _yaw))))

(event Input|ActionEvents|InputActionZoomIN
  (params (Key :type Key%20Structure))
  (bind _camerapawnref (Variables|References|GetCameraPawnRef))
  (bind _springarm (Variables|/Game/MyRTS/Blueprints/CameraPawn.CameraPawn_C|GetSpringArm _camerapawnref))
  ;[1 1 1] Zoom In/Out
  (:Pressed
    (Variables|/Script/Engine.SpringArmComponent|SetTargetArmLength _springarm (Math|Float|Clamp(Float) (- (Variables|/Script/Engine.SpringArmComponent|GetTargetArmLength _springarm) (Variables|Default|GetZoomSensitibity)) 5e+02 (Variables|Default|GetMaxArmDistance)))))

(event Input|ActionEvents|InputActionZoomOut
  (params (Key :type Key%20Structure))
  (bind _camerapawnref (Variables|References|GetCameraPawnRef))
  (bind _springarm (Variables|/Game/MyRTS/Blueprints/CameraPawn.CameraPawn_C|GetSpringArm _camerapawnref))
  ;[1 1 1] Zoom In/Out
  (:Pressed
    (Variables|/Script/Engine.SpringArmComponent|SetTargetArmLength _springarm (Math|Float|Clamp(Float) (+ (Variables|Default|GetZoomSensitibity) (Variables|/Script/Engine.SpringArmComponent|GetTargetArmLength _springarm)) 5e+02 (Variables|Default|GetMaxArmDistance)))))

(event Input|ActionEvents|InputActionZoomReset
  (params (Key :type Key%20Structure))
  (bind _camerapawnref (Variables|References|GetCameraPawnRef))
  ;[1 1 1] ZoomReset
  (:Pressed
    (Variables|/Script/Engine.SpringArmComponent|SetTargetArmLength (Variables|/Game/MyRTS/Blueprints/CameraPawn.CameraPawn_C|GetSpringArm _camerapawnref) (Variables|/Game/MyRTS/Blueprints/CameraPawn.CameraPawn_C|GetArmLenghtDefault _camerapawnref))))

(event Input|ActionEvents|InputActionDeselect
  (params (Key :type Key%20Structure))
  (:Pressed
    (if (Variables|Default|GetBuildModeActive)
      (Default|KillGhost (Variables|References|GetGhostBuildingRef))
      (Variables|Default|SetBuildModeActive false))))

(event Input|ActionEvents|InputActionRotateBuildingRight
  (params (Key :type Key%20Structure))
  (bind _ghostbuildingref (Variables|References|GetGhostBuildingRef))
  (bind _returnvalue (Transformation|GetActorRotation _ghostbuildingref))
  (bind (_roll _pitch _yaw) (Math|Rotator|BreakRotator _returnvalue))
  ;[1 1 1] Left Mouse Button
  (:Pressed
    (if (and (Variables|Default|GetBuildModeActive) (Utilities|IsValid _ghostbuildingref))
      (Transformation|SetActorRotation _ghostbuildingref (Math|Rotator|MakeRotator _roll _pitch (- _yaw (Variables|Default|GetBuiliduingRotationRATE)))))))

(event Input|ActionEvents|InputActionRotateBuildingLeft
  (params (Key :type Key%20Structure))
  (bind _ghostbuildingref (Variables|References|GetGhostBuildingRef))
  (bind _returnvalue (Transformation|GetActorRotation _ghostbuildingref))
  (bind (_roll _pitch _yaw) (Math|Rotator|BreakRotator _returnvalue))
  ;[1 1 1] Left Mouse Button
  (:Pressed
    (if (and (Variables|Default|GetBuildModeActive) (Utilities|IsValid _ghostbuildingref))
      (Transformation|SetActorRotation _ghostbuildingref (Math|Rotator|MakeRotator _roll _pitch (+ _yaw (Variables|Default|GetBuiliduingRotationRATE)))))))

(event Input|AxisEvents|InputAxisMoveForward
  (params (AxisValue :type Float%20%28single-precision%29))
  ;[1 1 1] Movement X
  (if (not (Variables|Default|GetDisableCamNav))
    (Transformation|SetActorTransform (Variables|References|GetCameraPawnRef) (Utilities|MouvementX (CallFunction|MovementSpeedCalculation) (Variables|Default|GetFastMoveMultiplier) AxisValue (Variables|References|GetCameraPawnRef)))))

(event Input|AxisEvents|InputAxisMoveRight
  (params (AxisValue :type Float%20%28single-precision%29))
  (bind _movesentitivity (CallFunction|MovementSpeedCalculation))
  (bind _camerapawnref (Variables|References|GetCameraPawnRef))
  (bind _fastmovemultiplier (Variables|Default|GetFastMoveMultiplier))
  (bind _transform (Utilities|MouvementY AxisValue _movesentitivity _fastmovemultiplier _camerapawnref))
  (bind (_location _rotation _scale) (Math|Transform|BreakTransform _transform))
  (bind (_x _y) (Math|Vector|BreakVector _location))
  ;[1 1 1] Movement Y
  (if (not (Variables|Default|GetDisableCamNav))
    (Transformation|SetActorTransform (Variables|References|GetCameraPawnRef) (Math|Transform|MakeTransform (Math|Vector|MakeVector _x _y 2e+02) _rotation _scale))))

(event Input|MouseEvents|MouseY
  (params (AxisValue :type Float%20%28single-precision%29))
  ;[1 1 1] EdgeMovement
  (if (not (Variables|Default|GetDisableCamNav))
    (Utilities|ScreenEdgeMovement) ; enters at MouseY
  ))

(event Input|MouseEvents|MouseX
  (params (AxisValue :type Float%20%28single-precision%29))
  (bind _camerapawnref (Variables|References|GetCameraPawnRef))
  (bind _returnvalue (Transformation|GetActorRotation _camerapawnref))
  (bind (_roll _pitch _yaw) (Math|Rotator|BreakRotator _returnvalue))
  ;[1 1 1] Pan X
  (Utilities|FlowControl|Gate true
    (:Exit
      (Transformation|SetActorRotation (Variables|References|GetCameraPawnRef) (Math|Rotator|MakeRotator _roll _pitch (+ (* (Variables|Default|GetPanSensitivity) AxisValue) _yaw))))))

(event Input|MouseEvents|MouseY
  (params (AxisValue :type Float%20%28single-precision%29))
  (bind _camerapawnref (Variables|References|GetCameraPawnRef))
  (bind _returnvalue (Transformation|GetActorRotation _camerapawnref))
  (bind (_roll _pitch _yaw) (Math|Rotator|BreakRotator _returnvalue))
  ;[1 1 1] Pan Y
  (Utilities|FlowControl|Gate true
    (:Exit
      (Transformation|SetActorRotation (Variables|References|GetCameraPawnRef) (Math|Rotator|MakeRotator _roll (Math|Float|Clamp(Float) (+ (* (Variables|Default|GetPanSensitivity) AxisValue) _pitch) -15.0 45.0) _yaw)))))

(event Input|MouseEvents|MouseX
  (params (AxisValue :type Float%20%28single-precision%29))
  ;[1 1 1] EdgeMovement
  (if (not (Variables|Default|GetDisableCamNav))
    (bind (_deltaxspeed _deltayspeed) (Utilities|ScreenEdgeMovement))
    (Transformation|AddActorLocalOffset (Variables|References|GetCameraPawnRef) (Math|Vector|MakeVector _deltaxspeed _deltayspeed 0.0) true false)))

(event Input|KeyboardEvents|LeftShift
  (params (Key :type Key%20Structure))
  ;[1 1 1] Move Multiplier
  (:Pressed
    (Variables|Default|SetFastMoveMultiplier 2.0))
  (:Released
    (Variables|Default|SetFastMoveMultiplier 1.0)))

(event Input|MouseEvents|LeftMouseButton
  (params (Key :type Key%20Structure))
  ;[1 1 1] Left Mouse Button
  (:Pressed
    (if (|VerifyAsPlaceable)
      (bind _constuctuionstruc (Default|GetConstructionStruct (Variables|References|GetGhostBuildingRef)))
      (Default|QueueConstruction (Variables|References|GetConstrucionManagerRef) _constuctuionstruc)
      (Default|KillGhost (Variables|References|GetGhostBuildingRef)))))

(event Input|KeyboardEvents|V
  (params (Key :type Key%20Structure))
  (bind _self self)
  (bind _location (CallFunction|SetCursrorWordPosition _self 1e+04))
  (:Pressed
    (Game|SpawnActorfromClass "/Game/MyRTS/Blueprints/NPC_BP.NPC_BP_C" (Math|Transform|MakeTransform (Math|Vector|MakeVector (.x _location) (.y _location) 186.0)) "AdjustIfPossibleButDontSpawnIfColliding" 0 0)))

(fn ConstructionScript)

(fn MovementSpeedCalculation
  (return (Math|Float|Clamp(Float) (/ (Variables|/Script/Engine.SpringArmComponent|GetTargetArmLength (Variables|/Game/MyRTS/Blueprints/CameraPawn.CameraPawn_C|GetSpringArm (Variables|References|GetCameraPawnRef))) 1e+02) 5.0 2e+01)))

(fn SetSightDistance
  (return (+ (Variables|Default|GetSightDistance) (Variables|/Script/Engine.SpringArmComponent|GetTargetArmLength (Variables|/Game/MyRTS/Blueprints/CameraPawn.CameraPawn_C|GetSpringArm (Variables|References|GetCameraPawnRef))))))

(fn SetCalendar
  (params (Date :type Array%20of%20Integers))
  (return false))

(fn SetClock
  (params (Time :type Array%20of%20Integers))
  (return false))