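; NPC Blueprint that gives each character a random gender, matching body color and name.
; The construction script calls RandomNPCFeatures, which creates a dynamic material instance on the mesh and sets its BodyColor from the rolled gender.
; GetRandomName picks a random entry from the male or female name enum as a string, stored with the gender in MyProfile.
; The event graph holds no active logic.
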(event EventBeginPlay)

(event Collision|EventActorBeginOverlap
  (params (OtherActor :type Actor%20Object%20Reference)))

(event EventTick
  (params (DeltaSeconds :type Float%20%28single-precision%29)))

(fn ConstructionScript
  (CallFunction|RandomNPCFeatures))

(fn RandomNPCFeatures
  (bind _returnvalue (Rendering|Material|CreateDynamicMaterialInstance (Variables|Character|GetMesh) 0 "/Game/Mannequin/Character/Materials/M_UE4Man_Body_Inst.M_UE4Man_Body_Inst" "None" :!class /Script/Engine.PrimitiveComponent))
  (LocalVariables|SetMaterialInstance _returnvalue)
  (if (Utilities|Enum|Equal(Enum) (Utilities|Enum|ByteToEnumNPCSexType_ENUM (Math|Conversions|ToByte(Integer) (Math|Random|RandomIntegerinRange 0 1))) "NewEnumerator0")
    (Rendering|Material|SetVectorParameterValue (LocalVariables|GetMaterialInstance) "BodyColor" (LocalVariables|GetMaleColor) :!class /Script/Engine.MaterialInstanceDynamic)
    (bind _name (CallFunction|GetRandomName "NewEnumerator0"))
    (Variables|Default|SetMyProfile (Utilities|Struct|MakeNPCProfile_Struct _name "NewEnumerator0"))
    (else
      (Rendering|Material|SetVectorParameterValue (LocalVariables|GetMaterialInstance) "BodyColor" (LocalVariables|GetFemaleColor) :!class /Script/Engine.MaterialInstanceDynamic)
      (bind _name_2 (CallFunction|GetRandomName "NewEnumerator1"))
      (Variables|Default|SetMyProfile (Utilities|Struct|MakeNPCProfile_Struct _name_2 "NewEnumerator1")))))

(fn GetRandomName
  (params (Gender :type NPCSexType_ENUM%20Enum :default "NewEnumerator0"))
  (if (Utilities|Enum|Equal(Enum) Gender "NewEnumerator0")
    (return (Utilities|String|EnumtoString (Utilities|Enum|LiteralenumNPCName_Male (Utilities|Enum|ByteToEnumNPCName_Male (Math|Conversions|ToByte(Integer) (Math|Random|RandomIntegerinRange 0 (- (|GetNumEnumEntries) 1)))))))
    (else
      (return (Utilities|String|EnumtoString (Utilities|Enum|LiteralenumNPCName_Female (Utilities|Enum|ByteToEnumNPCName_Female (Math|Conversions|ToByte(Integer) (Math|Random|RandomIntegerinRange 0 (- (|GetNumEnumEntries) 1))))))))))