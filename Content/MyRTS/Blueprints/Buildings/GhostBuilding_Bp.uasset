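; Placement preview ghost for RTS buildings, toggling the controller's build mode while active.
; ConstrucBuilding briefly spawns the building to read its mesh, proxy and work hours, then activates the ghost.
; A gated Tick grid-snaps it to the cursor position, swapping to an error material on overlap or excessive slope.
; Slope checks line-trace corners and center, box-tracing to adjust height; GetConstructionStruct packages the placement data.
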(event Custom|OnSpawn
  (params (DisplayMesh :type Static%20Mesh%20Object%20Reference) (BuidlingClass :type Building%20Master%20BP%20Class%20Reference) (ConstrucionProxy :type Construction%20Proxy%20Class%20Reference) (WorkHours :type Float%20%28single-precision%29))
  (bind _arrow (Variables|Default|GetArrow))
  ;[1 1 1] OnSpawn
  (if (not (Variables|Default|GetIsActive))
    (Variables|Default|SetConstructionProxy ConstrucionProxy)
    (Variables|Default|SetBuildingClass BuidlingClass)
    (Variables|Default|SetWorkHoursRequired WorkHours)
    (Variables|Default|SetDisplayMesh DisplayMesh)
    (Variables|Default|SetIsActive true)
    (Variables|/Game/MyRTS/Blueprints/CameraPawnController.CameraPawnController_C|SetBuildModeActive (Variables|Default|GetControllerRef) true)
    (Components|StaticMesh|SetStaticMesh (Variables|Default|GetGhostBuilding_Mesh) (Variables|Default|GetDisplayMesh))
    (CallFunction|OpenTickGate)
    (CallFunction|SetMaterialOverlapping (not (Variables|Default|GetIsOverlapping)))
    (bind _output_get (Variables|Default|SetExtent (.BoxExtent (Collision|GetComponentBounds (Variables|Default|GetGhostBuilding_Mesh)))))
    (Transformation|SetRelativeLocation _arrow (Math|Vector|MakeVector (.x _output_get) 0.0 0.0) false false)
    (Development|SetHiddeninGame _arrow false false)))

(event Custom|KillGhost
  ;[1 1 1] KillGhost
  (Variables|Default|SetConstructionProxy 0)
  (Variables|Default|SetBuildingClass 0)
  (CallFunction|CloseTickGate)
  (Variables|Default|SetDisplayMesh 0)
  (Variables|Default|SetIsActive false)
  (Variables|/Game/MyRTS/Blueprints/CameraPawnController.CameraPawnController_C|SetBuildModeActive (Variables|Default|GetControllerRef) false)
  (Components|StaticMesh|SetStaticMesh (Variables|Default|GetGhostBuilding_Mesh) (Variables|Default|GetDisplayMesh))
  (Transformation|SetActorRotation "0, 0, 0")
  (Development|SetHiddeninGame (Variables|Default|GetArrow) true false)
  (CallFunction|SetBuildingCollisionBox (Variables|Default|GetCollision) (Variables|Default|GetGhostBuilding_Mesh)))

(event Custom|OpenTickGate
  (bind _overlapping (CallFunction|CheckOverlap))
  ;[1 1 1] Tick
  (Utilities|FlowControl|Gate true) ; enters at Open
)

(event Custom|CloseTickGate
  (bind _overlapping (CallFunction|CheckOverlap))
  ;[1 1 1] Tick
  (Utilities|FlowControl|Gate true) ; enters at Close
)

(event Custom|SetMaterialOverlapping
  (params (IsError :type Boolean))
  (bind _ghostbuilding_mesh (Variables|Default|GetGhostBuilding_Mesh))
  ;[1 1 1] SetMaterialOverlapping
  (if (not (Math|Boolean|Equal(Boolean) IsError (Variables|Default|GetIsOverlapping)))
    (bind _output_get (Variables|Default|SetIsOverlapping IsError))
    (if _output_get
      (Rendering|Material|SetMaterial _ghostbuilding_mesh 0 "/Game/Materials/GhostError_M_Inst.GhostError_M_Inst")
      (else
        (Rendering|Material|SetMaterial _ghostbuilding_mesh 0 "/Game/Materials/Ghost_M_Inst.Ghost_M_Inst")))))

(event EventBeginPlay)

(event EventConstrucBuilding
  (params (MainBuilding :type Building%20Master%20BP%20Class%20Reference))
  ;[1 1 1] ConstrucBuilding
  (bind _returnvalue (Game|SpawnActorfromClass MainBuilding (Math|Transform|MakeTransform "0, 0, 0") "AlwaysSpawn" 0 (Variables|Default|GetControllerRef) 0))
  (Utilities|FlowControl|Sequence
    (:then_0
      (bind _asbuilding_master_bp (Utilities|Casting|CastToBuildingMaster_BPClass MainBuilding))
      (CallFunction|KillGhost)
      (CallFunction|OnSpawn (Variables|/Game/MyRTS/Blueprints/Buildings/BuildingMaster_BP.BuildingMaster_BP_C|GetDisplayMesh _returnvalue) _asbuilding_master_bp (Variables|/Game/MyRTS/Blueprints/Buildings/BuildingMaster_BP.BuildingMaster_BP_C|GetConstructionProxy _returnvalue) (Variables|/Game/MyRTS/Blueprints/Buildings/BuildingMaster_BP.BuildingMaster_BP_C|GetConstructionTime _returnvalue)))
    (:then_1
      (Actor|DestroyActor _returnvalue))))

(event Collision|EventActorBeginOverlap
  (params (OtherActor :type Actor%20Object%20Reference)))

(event EventTick
  (params (DeltaSeconds :type Float%20%28single-precision%29))
  (bind _overlapping (CallFunction|CheckOverlap))
  ;[1 1 1] Tick
  (Utilities|FlowControl|Gate true
    (:Exit
      (Transformation|SetActorLocation self (CallFunction|SetGridSnapVector) false false)
      (if _overlapping
        (CallFunction|SetMaterialOverlapping _overlapping)
        (else
          (bind _badlocation (CallFunction|CalculateSlope))
          (CallFunction|SetMaterialOverlapping _badlocation))))))

(fn ConstructionScript)

(fn SetGridSnapVector
  (bind _cursorworldpostion (Variables|Default|GetCursorWorldPostion))
  (bind _gridsize (Variables|Default|GetGridSize))
  (return (Math|Vector|MakeVector (CallFunction|GridSnap (.x _cursorworldpostion) _gridsize) (CallFunction|GridSnap (.y _cursorworldpostion) _gridsize) (CallFunction|GridSnap (.z _cursorworldpostion) _gridsize))))

(fn SetCursorPosition
  (params (CursorLocation :type Vector))
  (Variables|Default|SetCursorWorldPostion CursorLocation)
  (return))

(fn NewFunction0)

(fn GetConstructionStruct
  (return (Utilities|Struct|MakeConstruction_Struc (Variables|Default|GetBuildingClass) (Variables|Default|GetConstructionProxy) (Math|Transform|MakeTransform (Transformation|GetActorLocation) (Transformation|GetActorRotation)) (Variables|Default|GetDisplayMesh) (Variables|Default|GetWorkHoursRequired))))

(fn CheckOverlap
  (return (> (Utilities|Array|Length (Collision|GetOverlappingActors "/Script/Engine.Actor" :!class /Script/Engine.Actor)) 0)))

(fn CalculateSlope
  (bind (_actorlocation _forwardvector _rightvector) (CallFunction|GetVectors))
  (bind _actorlocation_2 (CallFunction|GetVectors))
  (bind _actorlocation_3 (CallFunction|GetVectors))
  (bind (_actorlocation_4 _forwardvector_2 _rightvector_2) (CallFunction|GetVectors))
  (bind (_actorlocation_5 _forwardvector_3 _rightvector_3) (CallFunction|GetVectors))
  (bind (_actorlocation_6 _forwardvector_4 _rightvector_4) (CallFunction|GetVectors))
  (bind _extent (Variables|Default|GetExtent))
  (bind _maxdiffrences (LocalVariables|GetMaxDiffrences))
  (bind _diffrences (LocalVariables|GetDiffrences))
  (bind (_indexofminvalue _minvalue) (Math|Float|MinOfFloatArray _diffrences))
  (bind (_indexofmaxvalue _maxvalue) (Math|Float|MaxOfFloatArray _diffrences))
  (Utilities|FlowControl|Sequence
    (:then_0
      (Utilities|FlowControl|Sequence
        (:then_0
          (bind _difference (CallFunction|SlopTrace (+ _actorlocation_4 (* (+ _forwardvector_2 _rightvector_2) (Variables|Default|GetExtent)))))
          (Utilities|Array|Add (LocalVariables|GetDiffrences) _difference))
        (:then_1
          (bind _difference_2 (CallFunction|SlopTrace (+ _actorlocation_5 (* (+ (* _forwardvector_3 -1.0) _rightvector_3) (Variables|Default|GetExtent)))))
          (Utilities|Array|Add (LocalVariables|GetDiffrences) _difference_2))
        (:then_2
          (bind _difference_3 (CallFunction|SlopTrace (+ _actorlocation_6 (* (+ _forwardvector_4 (* _rightvector_4 -1.0)) (Variables|Default|GetExtent)))))
          (Utilities|Array|Add (LocalVariables|GetDiffrences) _difference_3))
        (:then_3
          (bind _difference_4 (CallFunction|SlopTrace (+ _actorlocation (* (+ (* _forwardvector -1.0) (* _rightvector -1.0)) (Variables|Default|GetExtent)))))
          (Utilities|Array|Add (LocalVariables|GetDiffrences) _difference_4))
        (:then_4
          (bind _difference_5 (CallFunction|SlopTrace (.ActorLocation (CallFunction|GetVectors))))
          (Utilities|Array|Add (LocalVariables|GetDiffrences) _difference_5))))
    (:then_1
      (if (and (> _indexofminvalue -1) (> _indexofmaxvalue -1))
        (bind (_outhit _returnvalue) (Collision|BoxTraceByChannel (+ _actorlocation_2 "0, 0,1000.000000") (- _actorlocation_2 "0,1000.000000, 0") (Math|Vector|MakeVector (.x _extent) (.y _extent) 1.0) "0, 0, 0" "TraceTypeQuery3" false 0 "None"))
        (if _returnvalue
          (Transformation|SetActorLocation (Math|Vector|MakeVector (.x _actorlocation_3) (.y _actorlocation_3) (.z (.ImpactPoint (Collision|BreakHitResult _outhit)))) false false))))
    (:then_2
      (return (or (> (Math|Float|Absolute(Float) _minvalue) _maxdiffrences) (> (Math|Float|Absolute(Float) _maxvalue) _maxdiffrences))))))

(fn GetVectors
  (bind _returnvalue (Transformation|GetActorRotation))
  (return (Transformation|GetActorLocation) (Math|Vector|GetForwardVector _returnvalue) (Math|Vector|GetRightVector _returnvalue)))

(fn SlopTrace
  (params (TraceLocation :type Vector))
  (bind _outhit (Collision|LineTraceByChannel (+ TraceLocation "0, 0,1000.000000") (- TraceLocation "0, 0,1000.000000") "TraceTypeQuery3" false 0 "None"))
  (return (- (.z (Transformation|GetActorLocation)) (.z (.ImpactPoint (Collision|BreakHitResult _outhit))))))

(fn GetIsOverlapping
  (return (Variables|Default|GetIsOverlapping)))

(fn SetCalendar
  (params (Date :type Array%20of%20Integers))
  (return false))

(fn SetClock
  (params (Time :type Array%20of%20Integers))
  (return false))